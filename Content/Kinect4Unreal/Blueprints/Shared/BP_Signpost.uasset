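; BP_Signpost is a signpost Blueprint in the Kinect4Unreal shared content that displays up to six lines of text: a title, a description and four further lines.
; Its construction script passes each string through an Update Text Component macro, which destroys the text render component for an empty string or otherwise sets its text.
; It then applies TextColour to the first five components, leaving the sixth uncoloured.
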(fn ConstructionScript
  (bind _title (Variables|Default|GetTitle))
  (bind _line4 (Variables|Default|GetLine4))
  (bind _line3 (Variables|Default|GetLine3))
  (bind _description (Variables|Default|GetDescription))
  (bind _line5 (Variables|Default|GetLine5))
  (bind _line6 (Variables|Default|GetLine6))
  (Utilities|FlowControl|Sequence ; Sequentially add each line's text
    (:then_0
      (if (== (Utilities|String|Len _title) 0)
        (Utilities|UpdateTextComponent (Variables|Default|GetTextRender1) _title :!label _label)
        (else
          (goto _label Text%20Remains%20To%20Update))))
    (:then_1
      (if (== (Utilities|String|Len _description) 0)
        (Utilities|UpdateTextComponent (Variables|Default|GetTextRender2) _description :!label _label_2)
        (else
          (goto _label_2 Text%20Remains%20To%20Update))))
    (:then_2
      (if (== (Utilities|String|Len _line3) 0)
        (Utilities|UpdateTextComponent (Variables|Default|GetTextRender3) _line3 :!label _label_3)
        (else
          (goto _label_3 Text%20Remains%20To%20Update))))
    (:then_3
      (if (== (Utilities|String|Len _line4) 0)
        (Utilities|UpdateTextComponent (Variables|Default|GetTextRender4) _line4 :!label _label_4)
        (else
          (goto _label_4 Text%20Remains%20To%20Update))))
    (:then_4
      (if (== (Utilities|String|Len _line5) 0)
        (Utilities|UpdateTextComponent (Variables|Default|GetTextRender5) _line5 :!label _label_5)
        (else
          (goto _label_5 Text%20Remains%20To%20Update))))
    (:then_5
      (if (== (Utilities|String|Len _line6) 0)
        (Utilities|UpdateTextComponent (Variables|Default|GetTextRender6) _line6 :!label _label_6)
        (else
          (goto _label_6 Text%20Remains%20To%20Update))))
    (:then_6
      (Rendering|Components|TextRender|SetTextRenderColor (Variables|Default|GetTextRender1) (Math|Conversions|ToColor(LinearColor) (Variables|Default|GetTextColour))))))