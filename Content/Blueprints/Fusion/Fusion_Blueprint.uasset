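; Fusion actor that feeds a Kinect avateering skeleton into a FusionPlant and outputs to a fused skeleton.
; On BeginPlay it looks up the poseable mesh among BPAvateeringPoseable's child components, registers it as a skeleton and sets FusedSkeleton as the output target.
; Each Tick runs the fusion and moves a Cube to the plant's test position to check the output.
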(event EventBeginPlay
  ;[1 1 1] Get Kinect Poseable Mesh
  (bind _poseablemeshchild (CallFunction|GetPoseableMesh (Variables|Default|GetBP_Avateering_Poseable)))
  (bind _asposeable_mesh_component (Utilities|Casting|CastToPoseableMeshComponent _poseablemeshchild))
  (Class|FusionPlant|AddSkeleton (Variables|Default|GetFusionPlant) _asposeable_mesh_component)
  ;[1 1 1] Set Target for Fused Skeleton
  (Class|FusionPlant|SetOutputTarget (Variables|Default|GetFusionPlant) (Variables|Default|GetFusedSkeleton)))

(event EventTick
  (params (DeltaSeconds :type Float%20%28single-precision%29))
  (bind _fusionplant (Variables|Default|GetFusionPlant))
  ;[1 1 1] Test output function
  (Class|FusionPlant|Fuse _fusionplant)
  (bind _returnvalue (Class|FusionPlant|GetTestPosition _fusionplant))
  (Transformation|SetWorldLocation (Variables|Default|GetCube) (Math|Vector|MakeVector (.X (Math|Vector4|BreakVector4 _returnvalue)) (.Y (Math|Vector4|BreakVector4 _returnvalue)) (.Z (Math|Vector4|BreakVector4 _returnvalue))) false false))

(fn ConstructionScript)

(fn GetPoseableMesh
  (params (ParentObj :type Child%20Actor%20Component%20Object%20Reference))
  (bind _children (Components|GetChildrenComponents ParentObj true))
  (for _index (range 0 (Utilities|Array|Length _children))
    (bind _asposeable_mesh_component (Utilities|Casting|CastToPoseableMeshComponent (Utilities|Array|Get(acopy) _children _index)))
    (return _asposeable_mesh_component)))